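; Player-driven armed car Blueprint, built on TankAiming and TankMovement components, with a health bar widget linked on BeginPlay.
; Input drives movement, camera gimbal and spring-arm aiming, and a toggle between two arm lengths, while throttle input switches brake and reverse light materials.
; Holding Fire runs a self-re-entering Gate and Delay loop for rapid fire.
; Hits from components named "Bullet" briefly flash body and panel materials.
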(event `self.ReceiveBeginPlay`
  (`TankAimingComponent.Initialise` (`self.TankAiming`) (`self.Barrel`) (`self.Turret`))
  (`TankMovementComponent.Initialise` (`self.TankMovement`) (`self.Left Track`) (`self.Right Track`))
  (`self.SetHealthBar`))

(event `InputAxis|AimAzimuth`
  (params (AxisValue :type "Float (single-precision)"))
  ;[1 1 1] Balistics Input Binding
  (`SceneComponent.K2_AddLocalRotation` (`self.Azimuth Gimbal`) (`KismetMathLibrary.MakeRotator` 0.0 0.0 (* AxisValue (`GameplayStatics.GetWorldDeltaSeconds`) 100.0)) false false))

(event `InputAction|ChangeCamera`
  (params (Key :type "Key Structure"))
  (bind _springarm (`self.SpringArm`))
  ;[1 1 1] Toggle Camera View
  (:`Pressed`
    (`/Engine/EditorBlueprintResources/StandardMacros.FlipFlop`
      (:`A`
        (set `SpringArmComponent.TargetArmLength` 1000.0 _springarm))
      (:`B`
        (set `SpringArmComponent.TargetArmLength` 0.0 _springarm)))))

(event `InputAxis|MoveForward`
  (params (AxisValue :type "Float (single-precision)"))
  (bind _backlight (`self.BackLight`))
  ;[1 1 1] Movement Input Binding
  ;[1 1 1] Turning ON/OFF/Reverse the Back lights
  (if (< AxisValue 0.0)
    (`PrimitiveComponent.SetMaterial` (`self.LeftRLight`) 0 "/Game/Content/Materials/Reverse.Reverse")
    (`PrimitiveComponent.SetMaterial` (`self.RightRLight`) 0 "/Game/Content/Materials/Reverse.Reverse")
    (`TankMovementComponent.IntendMoveForward` (`self.TankMovement`) AxisValue :!label _label)
    (else
      (`PrimitiveComponent.SetMaterial` (`self.LeftRLight`) 0 "/Game/Content/Materials/BackLightsOFF.BackLightsOFF")
      (`PrimitiveComponent.SetMaterial` (`self.RightRLight`) 0 "/Game/Content/Materials/BackLightsOFF.BackLightsOFF")
      (if (> AxisValue 0.0)
        (`PrimitiveComponent.SetMaterial` _backlight 0 "/Game/Content/Materials/BackLightsOFF.BackLightsOFF")
        (`PrimitiveComponent.SetMaterial` (`self.RightBLight`) 0 "/Game/Content/Materials/BackLightsOFF.BackLightsOFF")
        (`PrimitiveComponent.SetMaterial` (`self.LeftBLight`) 0 "/Game/Content/Materials/BackLightsOFF.BackLightsOFF")
        (goto _label)
        (else
          (`PrimitiveComponent.SetMaterial` _backlight 0 "/Game/Content/Materials/BackLightsON.BackLightsON")
          (`PrimitiveComponent.SetMaterial` (`self.RightBLight`) 0 "/Game/Content/Materials/BackLightsON.BackLightsON")
          (`PrimitiveComponent.SetMaterial` (`self.LeftBLight`) 0 "/Game/Content/Materials/BackLightsON.BackLightsON"))))))

(event `InputAxis|TurnRight`
  (params (AxisValue :type "Float (single-precision)"))
  ;[1 1 1] Movement Input Binding
  (`TankMovementComponent.IntendMoveRight` (`self.TankMovement`) AxisValue))

(event `InputAxis|AimElevation`
  (params (AxisValue :type "Float (single-precision)"))
  ;[1 1 1] Balistics Input Binding
  (`SceneComponent.K2_AddLocalRotation` (`self.SpringArm`) (`KismetMathLibrary.MakeRotator` 0.0 (* AxisValue (`GameplayStatics.GetWorldDeltaSeconds`) 100.0)) false false))

(event `InputAction|Fire`
  (params (Key :type "Key Structure"))
  ;[1 1 1] Rapid-fire
  (:`Pressed`
    (`|ExecutionSequence`
      (:`then_0`
        (goto _label_2 :!via `Open`))
      (:`then_1`
        (`/Engine/EditorBlueprintResources/StandardMacros.Gate` true :!label _label_2
          (:`Exit`
            (`TankAimingComponent.Fire` (`self.TankAiming`))
            (`KismetSystemLibrary.Delay` 0.04)
            (goto _label_2))))))
  (:`Released`
    (goto _label_2 :!via `Close`)))

(event `self.Tank.OnComponentHit`
  (params (HitComponent :type "PrimitiveComponent Object Reference") (OtherActor :type "Actor Object Reference") (OtherComp :type "PrimitiveComponent Object Reference") (NormalImpulse :type "Vector Structure") (Hit :type "HitResult Structure (by ref)"))
  (bind _tank (`self.Tank`))
  (if (`KismetStringLibrary.EqualEqual_StrStr` (`KismetSystemLibrary.GetObjectName` OtherComp) "Bullet")
    (`PrimitiveComponent.SetMaterial` (`self.Tank`) 3 "/Game/Content/Materials/Car/Hit.Hit")
    (`PrimitiveComponent.SetMaterial` (`self.Panel`) 0 "/Game/Content/Materials/BackLightsON.BackLightsON")
    (`PrimitiveComponent.SetMaterial` _tank 0 "/Game/Content/Materials/Car/Hit.Hit")
    (`KismetSystemLibrary.Delay` 0.2)
    (`PrimitiveComponent.SetMaterial` _tank 0 "/Game/Content/Materials/M_Glass.M_Glass")
    (`PrimitiveComponent.SetMaterial` (`self.Panel`) 0 "/Game/Content/Materials/M_Glass.M_Glass")
    (`PrimitiveComponent.SetMaterial` _tank 3 "/Game/Content/Materials/M_Glass.M_Glass")))

(fn `SetHealthBar`
  (bind _ashealth_bar (cast `/Game/UI/HealthBar` (`WidgetComponent.GetUserWidgetObject` (`self.Widget`))))
  (set `/Game/UI/HealthBar.Tank` self _ashealth_bar))

(fn `UserConstructionScript`)