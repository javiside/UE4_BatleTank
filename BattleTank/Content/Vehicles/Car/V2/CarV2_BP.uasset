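; Player-controlled car pawn that reuses tank aiming and movement components, initialised with barrel, turret and tracks on BeginPlay.
; Aim axes rotate an azimuth gimbal and spring arm, while a camera toggle flips arm length.
; Throttle input spins wheels, spawns smoke and swaps brake and reverse light materials around a dead zone.
; Holding Fire loops shots through a delayed gate, and bullet hits briefly flash glass and panel materials.
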(event `self.ReceiveBeginPlay`
  (`TankAimingComponent.Initialise` (`self.TankAiming`) (`self.Barrel`) (`self.Turret`))
  (`TankMovementComponent.Initialise` (`self.TankMovement`) (`self.Left Track`) (`self.Right Track`)))

(event `InputAxis|AimAzimuth`
  (params (AxisValue :type "Float (single-precision)"))
  ;[1 1 1] Balistics Input Binding
  (`SceneComponent.K2_AddLocalRotation` (`self.Azimuth Gimbal`) (`KismetMathLibrary.MakeRotator` 0.0 0.0 (* AxisValue (`GameplayStatics.GetWorldDeltaSeconds`) 100.0)) false false))

(event `InputAction|ChangeCamera`
  (params (Key :type "Key Structure"))
  (bind _springarm (`self.SpringArm`))
  ;[1 1 1] Toggle Camera View
  (:`Pressed`
    (`/Engine/EditorBlueprintResources/StandardMacros.FlipFlop`
      (:`A`
        (set `SpringArmComponent.TargetArmLength` 1000.0 _springarm))
      (:`B`
        (set `SpringArmComponent.TargetArmLength` 0.0 _springarm)))))

(event `InputAxis|AimElevation`
  (params (AxisValue :type "Float (single-precision)"))
  ;[1 1 1] Balistics Input Binding
  (`SceneComponent.K2_AddLocalRotation` (`self.SpringArm`) (`KismetMathLibrary.MakeRotator` 0.0 (* AxisValue (`GameplayStatics.GetWorldDeltaSeconds`) 100.0)) false false))

(event `InputAxis|MoveForward`
  (params (AxisValue :type "Float (single-precision)"))
  (bind _throw (`self.Throw`))
  ;[1 1 1] Movement Input Binding
  (bind _output_get (set `self.Throw` AxisValue))
  (if (> _output_get 0.16)
    ;;[1 1 1] Forward: rotate wheels, attach smoke and turn off lights
    (`SceneComponent.K2_AddLocalRotation` (`self.WheelBackRight`) (`KismetMathLibrary.MakeRotator` 0.0 (* _throw 10.0)) false false)
    (`SceneComponent.K2_AddLocalRotation` (`self.WheelFrontRight`) (`KismetMathLibrary.MakeRotator` 0.0 (* _throw 10.0)) false false)
    (`SceneComponent.K2_AddLocalRotation` (`self.WheelFrontLeft`) (`KismetMathLibrary.MakeRotator` 0.0 (* _throw -10.0)) false false)
    (`SceneComponent.K2_AddLocalRotation` (`self.WheelBackLeft`) (`KismetMathLibrary.MakeRotator` 0.0 (* _throw -10.0)) false false)
    (`PrimitiveComponent.SetMaterial` (`self.LeftReverseLight`) 0 "/Game/Content/Materials/BackLightsOFF.BackLightsOFF")
    (`PrimitiveComponent.SetMaterial` (`self.RightReverseLight`) 0 "/Game/Content/Materials/BackLightsOFF.BackLightsOFF")
    (`PrimitiveComponent.SetMaterial` (`self.BackLight`) 0 "/Game/Content/Materials/BackLightsOFF.BackLightsOFF")
    (`PrimitiveComponent.SetMaterial` (`self.RightTailLight`) 0 "/Game/Content/Materials/BackLightsOFF.BackLightsOFF")
    (`PrimitiveComponent.SetMaterial` (`self.LeftTailLight`) 0 "/Game/Content/Materials/BackLightsOFF.BackLightsOFF")
    (`GameplayStatics.SpawnEmitterAttached` "/Game/Content/Particles/Smokee.Smokee" (`self.WheelBackRight`))
    (`GameplayStatics.SpawnEmitterAttached` "/Game/Content/Particles/Smokee.Smokee" (`self.WheelFrontRight`))
    (`GameplayStatics.SpawnEmitterAttached` "/Game/Content/Particles/Smokee.Smokee" (`self.WheelBackLeft`))
    (`GameplayStatics.SpawnEmitterAttached` "/Game/Content/Particles/Smokee.Smokee" (`self.WheelFrontLeft`))
    (`TankMovementComponent.IntendMoveForward` (`self.TankMovement`) _throw :!label _label)
    (elif (< AxisValue -0.16)
      ;;[1 1 1] Backwards: rotate wheels, attach smoke and turn on reverse lights
      (`SceneComponent.K2_AddLocalRotation` (`self.WheelBackRight`) (`KismetMathLibrary.MakeRotator` 0.0 (* _throw 10.0)) false false)
      (`SceneComponent.K2_AddLocalRotation` (`self.WheelFrontRight`) (`KismetMathLibrary.MakeRotator` 0.0 (* _throw 10.0)) false false)
      (`SceneComponent.K2_AddLocalRotation` (`self.WheelBackLeft`) (`KismetMathLibrary.MakeRotator` 0.0 (* _throw -10.0)) false false)
      (`SceneComponent.K2_AddLocalRotation` (`self.WheelFrontLeft`) (`KismetMathLibrary.MakeRotator` 0.0 (* _throw -10.0)) false false)
      (`PrimitiveComponent.SetMaterial` (`self.LeftReverseLight`) 0 "/Game/Content/Materials/Reverse.Reverse")
      (`PrimitiveComponent.SetMaterial` (`self.RightReverseLight`) 0 "/Game/Content/Materials/Reverse.Reverse")
      (`GameplayStatics.SpawnEmitterAttached` "/Game/Content/Particles/Smokee.Smokee" (`self.WheelBackLeft`))
      (`GameplayStatics.SpawnEmitterAttached` "/Game/Content/Particles/Smokee.Smokee" (`self.WheelFrontLeft`))
      (`GameplayStatics.SpawnEmitterAttached` "/Game/Content/Particles/Smokee.Smokee" (`self.WheelBackRight`))
      (`GameplayStatics.SpawnEmitterAttached` "/Game/Content/Particles/Smokee.Smokee" (`self.WheelFrontRight`))
      (goto _label)
      (else
        ;;[1 1 1] Stop: stop wheels and turn on lights
        (`PrimitiveComponent.SetMaterial` (`self.LeftReverseLight`) 0 "/Game/Content/Materials/BackLightsOFF.BackLightsOFF")
        (`PrimitiveComponent.SetMaterial` (`self.RightReverseLight`) 0 "/Game/Content/Materials/BackLightsOFF.BackLightsOFF")
        (`PrimitiveComponent.SetMaterial` (`self.LeftTailLight`) 0 "/Game/Content/Materials/BackLightsON.BackLightsON")
        (`PrimitiveComponent.SetMaterial` (`self.BackLight`) 0 "/Game/Content/Materials/BackLightsON.BackLightsON")
        (`PrimitiveComponent.SetMaterial` (`self.RightTailLight`) 0 "/Game/Content/Materials/BackLightsON.BackLightsON")))))

(event `InputAction|Fire`
  (params (Key :type "Key Structure"))
  ;[1 1 1] Rapid-Fire
  (:`Pressed`
    (`|ExecutionSequence`
      (:`then_0`
        (goto _label_2 :!via `Open`))
      (:`then_1`
        (`/Engine/EditorBlueprintResources/StandardMacros.Gate` true :!label _label_2
          (:`Exit`
            (`TankAimingComponent.Fire` (`self.TankAiming`))
            (`KismetSystemLibrary.Delay` 0.04)
            (goto _label_2))))))
  (:`Released`
    (goto _label_2 :!via `Close`)))

(event `InputAxis|TurnRight`
  (params (AxisValue :type "Float (single-precision)"))
  ;[1 1 1] Movement Input Binding
  (`TankMovementComponent.IntendMoveRight` (`self.TankMovement`) AxisValue))

(event `self.Tank.OnComponentHit`
  (params (HitComponent :type "PrimitiveComponent Object Reference") (OtherActor :type "Actor Object Reference") (OtherComp :type "PrimitiveComponent Object Reference") (NormalImpulse :type "Vector Structure") (Hit :type "HitResult Structure (by ref)"))
  (bind _glasswindow (`self.GlassWindow`))
  (bind _glasscover (`self.GlassCover`))
  (bind _panel (`self.Panel`))
  (if (`KismetStringLibrary.EqualEqual_StrStr` (`KismetSystemLibrary.GetObjectName` OtherComp) "Bullet")
    (`PrimitiveComponent.SetMaterial` _glasswindow 0 "/Game/Content/Materials/Car/Hit.Hit")
    (`PrimitiveComponent.SetMaterial` _panel 0 "/Game/Content/Materials/BackLightsON.BackLightsON")
    (`PrimitiveComponent.SetMaterial` _glasscover 0 "/Game/Content/Materials/Car/Hit.Hit")
    (`KismetSystemLibrary.Delay` 0.2)
    (`PrimitiveComponent.SetMaterial` _glasswindow 0 "/Game/Content/Materials/Car/Glass.Glass")
    (`PrimitiveComponent.SetMaterial` _panel 0 "/Game/Content/Materials/M_Glass.M_Glass")
    (`PrimitiveComponent.SetMaterial` _glasscover 0 "/Game/Content/Materials/M_Glass.M_Glass")))

(fn `UserConstructionScript`)